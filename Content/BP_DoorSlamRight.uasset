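; Door actor that slams back and forth on its own, starting at BeginPlay.
; BeginPlay derives an end point from the start location using a fixed X shift and a negative Y shift of MoveDistance.
; The OpenCloseSlamDoor timeline lerps the actor between both points without sweep.
; On finish, a FlipFlop alternates Play and Reverse, looping the motion endlessly without any trigger.
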(event `self.ReceiveBeginPlay`
  (bind _output_get (set `self.StartLocation` (`self.K2_GetActorLocation`)))
  (set `self.EndLocation` (`KismetMathLibrary.MakeVector` (+ (.x _output_get) 80.0) (- (.y _output_get) (`self.MoveDistance`)) (.z _output_get)))
  (bind (_direction _door) (`Timeline|openClose SlamDoor` :!via `PlayFromStart` :!label _label)
    (:`Update`
      (`self.K2_SetActorLocation` (`KismetMathLibrary.VLerp` (`self.StartLocation`) (`self.EndLocation`) _door)))
    (:`Finished`
      (`/Engine/EditorBlueprintResources/StandardMacros.FlipFlop`
        (:`A`
          (goto _label))
        (:`B`
          (goto _label :!via `Reverse`))))))

(fn `UserConstructionScript`)