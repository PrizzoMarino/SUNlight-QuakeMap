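; BP_Piston is a piston actor that moves its Piston component along relative Z by MoveDistance when play begins.
; The MovePiston timeline drives a swept lerp from the stored start location to the offset position.
; A one-second Delay followed by Reverse hangs off the timeline's Update rather than Finished, so reversal is timed from update ticks, not the end of the stroke.
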(event `self.ReceiveBeginPlay`
  (set `self.StartLocation` (`SceneComponent.RelativeLocation` (`self.Piston`)))
  (bind (_direction _movepiston) (`Timeline|MovePiston` :!label _label)
    (:`Update`
      (`SceneComponent.K2_SetRelativeLocation` (`self.Piston`) (`KismetMathLibrary.VLerp` (`self.StartLocation`) (+ (`self.StartLocation`) (`KismetMathLibrary.MakeVector` 0.0 0.0 (`self.MoveDistance`))) _movepiston) true false)
      (`KismetSystemLibrary.Delay` 1.0)
      (goto _label :!via `Reverse`))))

(fn `UserConstructionScript`)