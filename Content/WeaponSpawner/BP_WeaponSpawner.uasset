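; Rotating weapon pickup that gives the overlapping first-person character a Pistol, SMG, Launcher or AR, chosen by the spawner's actor tag.
; Box overlap calls GiveWeapon, which hides the pickup and disables collision for a delay, then restores it.
; Only after that delay does it spawn the weapon and attach it to the character's HandGrip_R socket.
; The Pistol branch reuses the SMG attach node, which targets the SMG reference.
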(event `GiveWeapon`
  (params (WeaponName :type String))
  (bind _mesh (`Character.Mesh` (`self.As BP First Person Character`)))
  (bind _mesh_2 (`Character.Mesh` (`self.As BP First Person Character`)))
  (`KismetSystemLibrary.PrintString` "Yoink")
  (`PrimitiveComponent.SetCollisionEnabled` (`self.Box`) "NoCollision")
  (`SceneComponent.SetVisibility` (`self.DefaultSceneRoot`) false true)
  (`KismetSystemLibrary.Delay` 5.0)
  (`PrimitiveComponent.SetCollisionEnabled` (`self.Box`) "QueryAndPhysics")
  (`SceneComponent.SetVisibility` (`self.DefaultSceneRoot`) true true)
  (`KismetSystemLibrary.PrintString` "poof")
  (if (`KismetStringLibrary.EqualEqual_StrStr` WeaponName "Pistol")
    (`|SpawnActorFromClass` "/Game/WeaponSpawner/BP_Pistol.BP_Pistol_C" (`SceneComponent.K2_GetComponentToWorld` _mesh_2) "AlwaysSpawn" "MultiplyWithRoot" null null)
    (`SceneComponent.K2_AttachToComponent` (`Actor.RootComponent` (stale _returnvalue)) _mesh_2 "HandGrip_R" "SnapToTarget" "SnapToTarget" "KeepRelative" true :!label _label)
    (elif (`KismetStringLibrary.EqualEqual_StrStr` WeaponName "SMG")
      (bind _returnvalue (`|SpawnActorFromClass` "/Game/WeaponSpawner/BP_SMG.BP_SMG_C" (`SceneComponent.K2_GetComponentToWorld` _mesh_2) "AlwaysSpawn" "MultiplyWithRoot" null null))
      (goto _label)
      (elif (`KismetStringLibrary.EqualEqual_StrStr` WeaponName "Launcher")
        (bind _returnvalue_2 (`|SpawnActorFromClass` "/Game/WeaponSpawner/BP_Launcher.BP_Launcher_C" (`SceneComponent.K2_GetComponentToWorld` _mesh) "AlwaysSpawn" "MultiplyWithRoot" null null))
        (`SceneComponent.K2_AttachToComponent` (`Actor.RootComponent` _returnvalue_2) _mesh "HandGrip_R" "SnapToTarget" "SnapToTarget" "KeepRelative" true)
        (elif (`KismetStringLibrary.EqualEqual_StrStr` WeaponName "AR")
          (bind _returnvalue_3 (`|SpawnActorFromClass` "/Game/WeaponSpawner/BP_AR.BP_AR_C" (`SceneComponent.K2_GetComponentToWorld` _mesh) "AlwaysSpawn" "MultiplyWithRoot" null null))
          (`SceneComponent.K2_AttachToComponent` (`Actor.RootComponent` _returnvalue_3) _mesh "HandGrip_R" "SnapToTarget" "SnapToTarget" "KeepRelative" true))))))

(event `self.ReceiveBeginPlay`
  (`AddComponent|NODE_AddRotatingMovementComponent-0`))

(event `self.ReceiveTick`
  (params (DeltaSeconds :type "Float (single-precision)")))

(event `self.Box.OnComponentBeginOverlap`
  (params (OverlappedComponent :type "PrimitiveComponent Object Reference") (OtherActor :type "Actor Object Reference") (OtherComp :type "PrimitiveComponent Object Reference") (OtherBodyIndex :type Integer) (bFromSweep :type Boolean) (SweepResult :type "HitResult Structure (by ref)"))
  (bind _asbp_first_person_character (cast `/Game/FirstPerson/Blueprints/BP_FirstPersonCharacter` OtherActor))
  (set `self.As BP First Person Character` _asbp_first_person_character)
  (if (`self.ActorHasTag` "Pistol")
    (bind _output_get (set `self.Tag` "Pistol"))
    (`self.GiveWeapon` _output_get)
    (elif (`self.ActorHasTag` "SMG")
      (bind _output_get_2 (set `self.Tag` "SMG"))
      (`self.GiveWeapon` _output_get_2)
      (elif (`self.ActorHasTag` "Launcher")
        (bind _output_get_3 (set `self.Tag` "Launcher"))
        (`self.GiveWeapon` _output_get_3)
        (elif (`self.ActorHasTag` "AR")
          (bind _output_get_4 (set `self.Tag` "AR"))
          (`self.GiveWeapon` _output_get_4))))))

(fn `UserConstructionScript`)