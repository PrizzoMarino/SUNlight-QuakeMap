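; Game mode that spawns and respawns players at random Player Start locations.
; BeginPlay caches every PlayerStart actor in the level, and the ChoosePlayerStart override returns a random entry from that array, without checking whether it is occupied.
; The RespawnPlayer event calls RestartPlayer on any valid controller passed to it.
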(event `RespawnPlayer`
  (params (Controller :type "Controller Object Reference"))
  (`/Engine/EditorBlueprintResources/StandardMacros.IsValid` Controller
    (:`Is Valid`
      (`self.RestartPlayer` Controller))))

(event `self.ReceiveBeginPlay`
  (bind _outactors (`GameplayStatics.GetAllActorsOfClass` "/Script/Engine.PlayerStart"))
  (set `self.PlayerStarts` _outactors))

(fn `ChoosePlayerStart`
  (params (Player :type "Controller Object Reference"))
  (returns (ReturnValue :type "Actor Object Reference"))
  (bind _playerstarts (`self.PlayerStarts`))
  (return (`|GetArrayItem` _playerstarts (`KismetMathLibrary.RandomIntegerInRange` 0 (- (`KismetArrayLibrary.Array_Length` _playerstarts) 1)))))

(fn `UserConstructionScript`)