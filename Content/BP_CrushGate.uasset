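; BP_CrushGate is a timed hazard that kills the first-person player caught inside its box during the crush window.
; BeginPlay runs an endless delay loop that briefly switches CanCrush on in each cycle.
; Box overlap events store or clear the BP_FirstPersonCharacter reference and inside flag.
; Tick checks both flags every frame, then sets PlayerDied and calls Die on that character.
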(event `self.ReceiveBeginPlay`
  (`KismetSystemLibrary.Delay` 1.8 :!label _label)
  (set `self.bCanCrush` true)
  (`KismetSystemLibrary.Delay` 0.4)
  (set `self.bCanCrush` false)
  (`KismetSystemLibrary.Delay` 1.7)
  (goto _label))

(event `self.ReceiveTick`
  (params (DeltaSeconds :type "Float (single-precision)"))
  (bind _player (`self.Player`))
  (if (and (`self.bCanCrush`) (`self.bPlayerInside`))
    (`/Engine/EditorBlueprintResources/StandardMacros.IsValid` _player
      (:`Is Valid`
        (set `/Game/FirstPerson/Blueprints/BP_FirstPersonCharacter.PlayerDied` true _player)
        (`/Game/FirstPerson/Blueprints/BP_FirstPersonCharacter.Die` _player)))))

(event `self.Box.OnComponentBeginOverlap`
  (params (OverlappedComponent :type "PrimitiveComponent Object Reference") (OtherActor :type "Actor Object Reference") (OtherComp :type "PrimitiveComponent Object Reference") (OtherBodyIndex :type Integer) (bFromSweep :type Boolean) (SweepResult :type "HitResult Structure (by ref)"))
  (bind _asbp_first_person_character (cast `/Game/FirstPerson/Blueprints/BP_FirstPersonCharacter` OtherActor))
  (set `self.Player` _asbp_first_person_character)
  (set `self.bPlayerInside` true))

(event `self.Box.OnComponentEndOverlap`
  (params (OverlappedComponent :type "PrimitiveComponent Object Reference") (OtherActor :type "Actor Object Reference") (OtherComp :type "PrimitiveComponent Object Reference") (OtherBodyIndex :type Integer))
  (cast `/Game/FirstPerson/Blueprints/BP_FirstPersonCharacter` OtherActor)
  (set `self.Player` null)
  (set `self.bPlayerInside` false))

(fn `UserConstructionScript`)