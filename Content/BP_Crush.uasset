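; BP_Crush is a crusher hazard meant to kill the first-person player standing inside it during its crush window.
; A looping Delay chain from BeginPlay briefly enables CanCrush each cycle, while Box overlap events track PlayerInside.
; Tick checks both flags, then sets PlayerDied and calls Die on its Owner cast to BP_FirstPersonCharacter, not on the overlapping actor.
; Debug prints report each state.
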(event `self.ReceiveBeginPlay`
  (`KismetSystemLibrary.Delay` 0.8 :!label _label)
  (bind _output_get (set `self.bCanCrush` true))
  (`KismetSystemLibrary.PrintString` (`KismetStringLibrary.Conv_BoolToString` _output_get))
  (`KismetSystemLibrary.Delay` 0.4)
  (bind _output_get_2 (set `self.bCanCrush` false))
  (`KismetSystemLibrary.PrintString` (`KismetStringLibrary.Conv_BoolToString` _output_get_2))
  (`KismetSystemLibrary.Delay` 0.8)
  (goto _label))

(event `self.ReceiveTick`
  (params (DeltaSeconds :type "Float (single-precision)"))
  (if (and (`self.bCanCrush`) (`self.bPlayerInside`))
    (`KismetSystemLibrary.PrintString` "Player died")
    (bind _asbp_first_person_character (cast `/Game/FirstPerson/Blueprints/BP_FirstPersonCharacter` (`self.GetOwner`)))
    (set `/Game/FirstPerson/Blueprints/BP_FirstPersonCharacter.PlayerDied` true _asbp_first_person_character)
    (`/Game/FirstPerson/Blueprints/BP_FirstPersonCharacter.Die` _asbp_first_person_character)
    (`KismetSystemLibrary.PrintString` "PLAYER HAS DIEDDD")))

(event `self.Box.OnComponentBeginOverlap`
  (params (OverlappedComponent :type "PrimitiveComponent Object Reference") (OtherActor :type "Actor Object Reference") (OtherComp :type "PrimitiveComponent Object Reference") (OtherBodyIndex :type Integer) (bFromSweep :type Boolean) (SweepResult :type "HitResult Structure (by ref)"))
  (cast `/Game/FirstPerson/Blueprints/BP_FirstPersonCharacter` OtherActor)
  (set `self.bPlayerInside` true))

(event `self.Box.OnComponentEndOverlap`
  (params (OverlappedComponent :type "PrimitiveComponent Object Reference") (OtherActor :type "Actor Object Reference") (OtherComp :type "PrimitiveComponent Object Reference") (OtherBodyIndex :type Integer))
  (cast `/Game/FirstPerson/Blueprints/BP_FirstPersonCharacter` OtherActor)
  (set `self.bPlayerInside` false))

(fn `UserConstructionScript`)